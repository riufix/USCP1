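; BP_LightingSystem spotlights whichever character is speaking during dialogue.
; On BeginPlay it finds the DialogSystem actor and binds to its read-dialog event dispatcher.
; Each dialog event hides the four character spotlights (Huguette, M. Pasteur, M. Rouget, M. Dupont), then shows the one matching the Speaker name string.
; An unmatched speaker name leaves all four lights off.
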(event `self.ReceiveBeginPlay`
  (bind _returnvalue (`GameplayStatics.GetActorOfClass` "/Game/USCP1/DialogSystem/DialogSystem.DialogSystem_C"))
  (add `/Game/USCP1/DialogSystem/DialogSystem.ED_OnReadDialog` _returnvalue (delegate `CE_MDR`)))

(event `CE_MDR`
  (params (Data :type "/Game/USCP1/DialogSystem/Data/S_DialogData Structure"))
  (bind (_dialogtype _speaker) (break `/Game/USCP1/DialogSystem/Data/S_DialogData` Data))
  (`SceneComponent.SetVisibility` (`SpotLight.SpotLightComponent` (`self.Huguette`)) false false)
  (`SceneComponent.SetVisibility` (`SpotLight.SpotLightComponent` (`self.M Pasteur`)) false false)
  (`SceneComponent.SetVisibility` (`SpotLight.SpotLightComponent` (`self.M Rouget`)) false false)
  (`SceneComponent.SetVisibility` (`SpotLight.SpotLightComponent` (`self.M Dupont`)) false false)
  (if (== _speaker "Huguette")
    (`SceneComponent.SetVisibility` (`SpotLight.SpotLightComponent` (`self.Huguette`)) true false)
    (elif (== _speaker "M. Pasteur")
      (`SceneComponent.SetVisibility` (`SpotLight.SpotLightComponent` (`self.M Pasteur`)) true false)
      (elif (== _speaker "M. Rouget")
        (`SceneComponent.SetVisibility` (`SpotLight.SpotLightComponent` (`self.M Rouget`)) true false)
        (elif (== _speaker "M. Dupont")
          (`SceneComponent.SetVisibility` (`SpotLight.SpotLightComponent` (`self.M Dupont`)) true false))))))

(fn `UserConstructionScript`)