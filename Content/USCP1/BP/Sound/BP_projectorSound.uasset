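; BP_projectorSound controls projector audio through its Audio component, which starts when the Onplay event is called.
; On BeginPlay it finds the DialogSystem actor and binds to its call-event dispatcher.
; A "Faidein" event pauses the audio, swaps in the end-of-chapter projector sound and binds to BP_PC_Player's skip-dialog dispatcher, which unpauses playback when fired.
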(event `On play`
  (`AudioComponent.Play` (`self.Audio`) 0.0))

(event `self.ReceiveBeginPlay`
  (bind _returnvalue (`GameplayStatics.GetActorOfClass` "/Game/USCP1/DialogSystem/DialogSystem.DialogSystem_C"))
  (set `self.faide in` _returnvalue)
  (bind _faide_in (`self.faide in`)
    (:`then`
      (add `/Game/USCP1/DialogSystem/DialogSystem.ED_OnCallEvent` _faide_in (delegate `CE_StopSound`)))
    (:`else`)))

(event `CE_StopSound`
  (params (EventName :type String))
  (bind _audio (`self.Audio`))
  (if (== EventName "Faidein")
    (`AudioComponent.SetPaused` _audio true)
    (`AudioComponent.SetSound` _audio (`self.Play projector End Chapter`))
    (bind _asbp_pc_player (cast `/Game/USCP1/BP/Exploration/BP_PC_Player` (`GameplayStatics.GetPlayerController` 0)))
    (add `/Game/USCP1/BP/Exploration/BP_PC_Player.ED_OnSkipDialog` _asbp_pc_player (delegate `CE_Resume`))))

(event `CE_Resume`
  (`AudioComponent.SetPaused` (`self.Audio`) false))

(fn `UserConstructionScript`)