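; Exploration player Blueprint that adds a camera vignette focus effect driven by dialog events.
; On BeginPlay it finds the DialogSystem actor and binds a handler to its call-event dispatcher, which passes an event name.
; "Focus" plays a timeline that animates the camera's post-process vignette intensity, and "StopFocus" reverses it from the end.
; A separate test event also triggers the reverse.
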(event `self.ReceiveBeginPlay`
  (bind _returnvalue (`GameplayStatics.GetActorOfClass` "/Game/USCP1/DialogSystem/DialogSystem.DialogSystem_C"))
  (add `/Game/USCP1/DialogSystem/DialogSystem.ED_OnCallEvent` _returnvalue (delegate `CE_CamFocus`)))

(event `CE_CamFocus`
  (params (EventName :type String))
  (if (== EventName "Focus")
    (bind (_direction _intensityprogression) (`Timeline|tl_CamVignette` :!via `PlayFromStart` :!label _label)
      (:`Update`
        (bind _camera (`self.Camera`)
          (:`then`
            (bind _structout (setmembers `PostProcessSettings` :`StructRef` (`CameraComponent.PostProcessSettings` _camera) :`VignetteIntensity` _intensityprogression :`DepthOfFieldVignetteSize` 200.0))
            (set `CameraComponent.PostProcessSettings` _structout _camera))
          (:`else`))))
    (elif (== EventName "StopFocus")
      (goto _label :!via `ReverseFromEnd`))))

(event `CE_test`
  (goto _label :!via `ReverseFromEnd`))

(fn `UserConstructionScript`)