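; Player controller Blueprint for exploration, handling enhanced input for camera look and character movement.
; On BeginPlay it adds the exploration mapping context to the local player's input subsystem, printing an error if that subsystem is invalid.
; The camera action feeds yaw and pitch to player character 0, and the movement action moves it along its actor right and forward vectors.
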(event `self.ReceiveBeginPlay`
  (bind _returnvalue (subsystem `EnhancedInputLocalPlayerSubsystem`))
  ;[1 1 1] Add IMC
  (`/Engine/EditorBlueprintResources/StandardMacros.IsValid` _returnvalue
    (:`Is Valid`
      (`EnhancedInputSubsystemInterface.AddMappingContext` _returnvalue "/Game/USCP1/Inputs/IMC_Exploration.IMC_Exploration" 0 (struct)))
    (:`Is Not Valid`
      (`KismetSystemLibrary.PrintString` "Invalid Input Local Player Subsystem"))))

(event `EnhancedInput|/Game/USCP1/Inputs/IA_ExplorationCamera`
  (params (ActionValue :type "Vector2D Structure") (ElapsedSeconds :type "Float (double-precision)") (TriggeredSeconds :type "Float (double-precision)") (InputAction :type "InputAction Object Reference" :default "/Game/USCP1/Inputs/IA_ExplorationCamera.IA_ExplorationCamera"))
  (bind _returnvalue (`GameplayStatics.GetPlayerCharacter` 0))
  ;[1 1 1] Camera
  (:`Triggered`
    (`Pawn.AddControllerYawInput` _returnvalue ActionValue_X)
    (`Pawn.AddControllerPitchInput` _returnvalue ActionValue_Y)))

(event `EnhancedInput|/Game/USCP1/Inputs/IA_ExplorationMovement`
  (params (ActionValue :type "Vector2D Structure") (ElapsedSeconds :type "Float (double-precision)") (TriggeredSeconds :type "Float (double-precision)") (InputAction :type "InputAction Object Reference" :default "/Game/USCP1/Inputs/IA_ExplorationMovement.IA_ExplorationMovement"))
  (bind _returnvalue (`GameplayStatics.GetPlayerCharacter` 0))
  (bind _returnvalue_2 (`GameplayStatics.GetPlayerCharacter` 0))
  ;[1 1 1] Movement
  (:`Triggered`
    (`Pawn.AddMovementInput` _returnvalue (`self.GetActorRightVector` _returnvalue) ActionValue_X false)
    (`Pawn.AddMovementInput` _returnvalue_2 (`self.GetActorForwardVector` _returnvalue_2) ActionValue_Y false)))

(fn `UserConstructionScript`)