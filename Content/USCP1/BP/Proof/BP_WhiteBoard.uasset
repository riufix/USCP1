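; Whiteboard Blueprint that controls which chapter's proof actors are active, driven by the dialog system.
; On BeginPlay it finds the DialogSystem, binds to its call event and disables the three chapter proof lists.
; CE_ResetChapter matches SpawnProof event names to enable one chapter's list and disable the others.
; EnableProofs toggles visibility, collision and tick, but returns inside its loop, affecting only each list's first actor.
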(event `self.ReceiveBeginPlay`
  ;[1 1 1] Get dialog system
  ;;[1 1 1] OUI C'EST MOCHE
  (bind _returnvalue (`GameplayStatics.GetActorOfClass` "/Game/USCP1/DialogSystem/DialogSystem.DialogSystem_C"))
  (set `self.DialogSystem` _returnvalue)
  (bind _dialogsystem (`self.DialogSystem`)
    (:`then`
      (add `/Game/USCP1/DialogSystem/DialogSystem.ED_OnCallEvent` _dialogsystem (`|CreateDelegate` :!event `CE_ResetChapter`))
      ;[1 1 1] Disable every proof
      (`self.EnableProofs` (`self.Chapter1_Proof`))
      (`self.EnableProofs` (`self.Chapter2_Proof`))
      (`self.EnableProofs` (`self.Chapter3_Proof`)))
    (:`else`)))

(event `CE_ResetChapter`
  (params (EventName :type String))
  ;[1 1 1] Spawn proofs when triggered in DS
  (if (== EventName "SpawnProof_1")
    (`self.EnableProofs` (`self.Chapter1_Proof`) true)
    (`self.EnableProofs` (`self.Chapter2_Proof`))
    (`self.EnableProofs` (`self.Chapter3_Proof`))
    (elif (== EventName "SpawnProof_2")
      (`self.EnableProofs` (`self.Chapter1_Proof`))
      (`self.EnableProofs` (`self.Chapter2_Proof`) true)
      (`self.EnableProofs` (`self.Chapter3_Proof`))
      (elif (== EventName "SpawnProof_3")
        (`self.EnableProofs` (`self.Chapter1_Proof`))
        (`self.EnableProofs` (`self.Chapter2_Proof`))
        (`self.EnableProofs` (`self.Chapter3_Proof`) true)))))

(fn `UserConstructionScript`)