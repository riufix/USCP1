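; BP_TestProof is a proof actor that can link to another proof and carry a cable component.
; AddNewCableComponent replaces any existing cable with a new short one, and AssignLink stores the linked proof.
; RemoveEveryCableComponent destroys the cables on itself and its linked proof, then clears the references on both sides.
; BeginPlay switches on the Proof value but runs no logic.
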(event `self.ReceiveBeginPlay`
  (switch `/Game/USCP1/Data/E_EvidenceList` (`self.Proof`)))

(fn `AddNewCableComponent`
  (returns (`Output Cable` :type "CableComponent Object Reference"))
  ;[1 1 1] Destroy / Create cable
  (bind _cablecomponent (`self.CableComponent`)
    (:`then`
      (`ActorComponent.K2_DestroyComponent` _cablecomponent))
    (:`else`
      _))
  (bind _returnvalue (`AddComponent|NODE_AddCableComponent-0`))
  ;[1 1 1] Cable properties
  (bind _output_get (set `self.CableComponent` _returnvalue))
  (set `CableComponent.CableLength` 1.0 _output_get)
  (return _output_get))

(fn `AssignLink`
  (params (Linked :type "/Game/USCP1/BP/Proof/BP_TestProof Object Reference"))
  (set `self.LinkedProof` Linked))

(fn `DestroyCableComponent`
  (bind _cablecomponent (`self.CableComponent`)
    (:`then`
      (`ActorComponent.K2_DestroyComponent` _cablecomponent))
    (:`else`
      _))
  (return))

(fn `RemoveEveryCableComponent`
  ;[1 1 1] Remove cable component
  (`self.DestroyCableComponent`)
  (bind _linkedproof (`self.LinkedProof`)
    (:`then`
      (`self.DestroyCableComponent` _linkedproof)
      ;[1 1 1] Eveyone forget their link
      (bind _linkedproof_2 (`self.LinkedProof`)
        (:`then`
          (set `/Game/USCP1/BP/Proof/BP_TestProof.LinkedProof` null _linkedproof_2))
        (:`else`
          _))
      (set `self.LinkedProof` null))
    (:`else`)))

(fn `UserConstructionScript`)