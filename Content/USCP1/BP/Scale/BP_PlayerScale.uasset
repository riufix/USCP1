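; BP_PlayerScale is an actor that acts as the player's scale, raising or lowering as the jury's opinion changes.
; On BeginPlay it binds to the jury-opinion event in GI_USCP1, stores its start position and attaches the linked objects so they move along.
; Each change plays a timeline that blends from the stored height fraction toward opinion/100, setting a Z offset between MinHeight and MaxHeight.
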(event `self.ReceiveBeginPlay`
  (bind _asgi_uscp1 (cast `/Game/USCP1/BP/GameMode/GI_USCP1` (`GameplayStatics.GetGameInstance`)))
  (add `/Game/USCP1/BP/GameMode/GI_USCP1.ED_OnChangeJuryOpinion` _asgi_uscp1 (delegate `CE_ChangeHeight`))
  (set `self.DefaultHeight` 0.5)
  (set `self.DefaultPosition` (`self.K2_GetActorLocation`))
  (for _array_element (`self.ObjectsToLink`)
    (`self.K2_AttachToActor` _array_element self "None" "KeepRelative" "KeepRelative" "KeepRelative" true)))

(event `CE_ChangeHeight`
  (params (NewOpinion :type "Float (double-precision)"))
  (bind (_defaultposition_x _defaultposition_y _defaultposition_z) (`KismetMathLibrary.BreakVector` (`self.DefaultPosition`)))
  ;[1 1 1] Change scale
  (set `self.GoTo` (/ NewOpinion 100.0))
  (bind (_direction _0_to_0_5) (`Timeline|Timeline` :!via `PlayFromStart`)
    (:`Update`
      (`self.K2_SetActorLocation` (`KismetMathLibrary.MakeVector` _defaultposition_x _defaultposition_y (+ _defaultposition_z (`KismetMathLibrary.Lerp` (`self.MinHeight`) (`self.MaxHeight`) (`KismetMathLibrary.Lerp` (`self.DefaultHeight`) (`self.GoTo`) _0_to_0_5))))))
    (:`Finished`
      (set `self.DefaultHeight` (`self.GoTo`)))))

(fn `UserConstructionScript`)