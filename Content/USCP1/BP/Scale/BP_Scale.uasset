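; BP_Scale is a balance scale prop that tips to show the jury's current opinion.
; On BeginPlay it caches the resting bucket and support transforms and binds to the jury opinion change dispatcher on GI_USCP1.
; After a four-second delay, a timeline blends from the previous normalized opinion to the new one, offsetting both buckets' heights and the support's pitch.
; The reached value becomes the next starting point.
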(event `self.ReceiveBeginPlay`
  (set `self.Default BL pos` (`SceneComponent.RelativeLocation` (`self.BucketL`)))
  (set `self.Default BR pos` (`SceneComponent.RelativeLocation` (`self.BucketR`)))
  (set `self.Default Support Rot` (`SceneComponent.RelativeRotation` (`self.Support`)))
  (set `self.DefaultProg` 0.5)
  (bind _asgi_uscp1 (cast `/Game/USCP1/BP/GameMode/GI_USCP1` (`GameplayStatics.GetGameInstance`)))
  (add `/Game/USCP1/BP/GameMode/GI_USCP1.ED_OnChangeJuryOpinion` _asgi_uscp1 (`|CreateDelegate` :!event `Change Bucket Position`)))

(event `Change Bucket Position`
  (params (NewJuryOpinion :type "Float (double-precision)"))
  (bind (_default_bl_pos_x _default_bl_pos_y _default_bl_pos_z) (`KismetMathLibrary.BreakVector` (`self.Default BL pos`)))
  (bind (_default_br_pos_x _default_br_pos_y _default_br_pos_z) (`KismetMathLibrary.BreakVector` (`self.Default BR pos`)))
  (bind (_default_support_rot_roll _default_support_rot_pitch _default_support_rot_yaw) (`KismetMathLibrary.BreakRotator` (`self.Default Support Rot`)))
  (set `self.Go To` (/ NewJuryOpinion 100.0))
  (`KismetSystemLibrary.Delay` 4.0)
  (bind (_direction _0_to_0_5) (`Timeline|Go To Pos` :!via `PlayFromStart`)
    (:`Update`
      (bind _returnvalue (`KismetMathLibrary.Lerp` (`self.DefaultProg`) (`self.Go To`) _0_to_0_5))
      (`SceneComponent.K2_SetRelativeLocation` (`self.BucketL`) (`KismetMathLibrary.MakeVector` _default_bl_pos_x _default_bl_pos_y (+ _default_bl_pos_z (`KismetMathLibrary.Lerp` (`self.BL Go Highest`) (`self.BL Go Lowest`) _returnvalue))) false false)
      (`SceneComponent.K2_SetRelativeLocation` (`self.BucketR`) (`KismetMathLibrary.MakeVector` _default_br_pos_x _default_br_pos_y (+ _default_br_pos_z (`KismetMathLibrary.Lerp` (`self.BR Highest`) (`self.BR Lowest`) _returnvalue))) false false)
      (`SceneComponent.K2_SetRelativeRotation` (`self.Support`) (`KismetMathLibrary.MakeRotator` _default_support_rot_roll (+ _default_support_rot_pitch (`KismetMathLibrary.Lerp` (`self.Support Rot L`) (`self.Support Rot R`) _returnvalue)) _default_support_rot_yaw) false false))
    (:`Finished`
      (set `self.DefaultProg` (`self.Go To`)))))

(fn `UserConstructionScript`)